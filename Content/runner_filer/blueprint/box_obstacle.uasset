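; Moving box obstacle for a runner game that kills the player on contact.
; On BeginPlay it stores its start location and plays the Movement_box timeline, which offsets the box from that point without sweep.
; Each timeline update also spawns the Game_over 2D sound and immediately destroys that audio component.
; An actor overlap casts the other actor to ThirdPersonCharacter and calls its DeathFunction.
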(event `self.ReceiveBeginPlay`
  (set `self.initial_location` (`self.K2_GetActorLocation`))
  (bind (_direction _newtrack_0) (`Timeline|movement_box` :!via `PlayFromStart`)
    (:`Update`
      (bind _returnvalue (`GameplayStatics.SpawnSound2D` "/Game/runner_filer/sound/game_over.game_over" 1.0 1.0 0.0 null))
      (`ActorComponent.K2_DestroyComponent` _returnvalue)
      (`self.K2_SetActorLocation` (+ (`self.initial_location`) _newtrack_0)))))

(event `self.ReceiveActorBeginOverlap`
  (params (OtherActor :type "Actor Object Reference"))
  (bind _asthird_person_character (cast `/Game/ThirdPersonBP/Blueprints/ThirdPersonCharacter` OtherActor))
  (`/Game/ThirdPersonBP/Blueprints/ThirdPersonCharacter.deathFunction` _asthird_person_character))

(fn `UserConstructionScript`)