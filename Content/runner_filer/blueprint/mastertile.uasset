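; Master tile for an endless runner, populating itself with road, water and train obstacles around the player's path.
; BeginPlay spawns the ocean, a randomly placed optional coin, chance-based cars, then staggered boards across five water rows, using chained delays.
; When the character overlaps Box, the game mode spawns another tile and adds multiplier-scaled points.
; Overlapping Box1 sends a train from a random side with a honk.
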(event `self.ReceiveBeginPlay`
  (`self.spawn_water`)
  (`self.Spawn money`)
  (`self.Spawn_top_car`)
  (`KismetSystemLibrary.Delay` 1.25)
  (`self.Spawn_top_car`)
  (`self.Spawn_bot_car`)
  (`KismetSystemLibrary.Delay` 1.5)
  (`self.Spawn_bot_car`)
  (`self.Spawn_bot_board`)
  (`KismetSystemLibrary.Delay` 0.75)
  (`self.Spawn_bot_board`)
  (`KismetSystemLibrary.Delay` 0.75)
  (`self.Spawn_bot_board`)
  (`self.Spawn_mid_board1`)
  (`KismetSystemLibrary.Delay` 0.75)
  (`self.Spawn_mid_board1`)
  (`KismetSystemLibrary.Delay` 0.75)
  (`self.Spawn_mid_board1`)
  (`self.Spawn_mid_board2`)
  (`KismetSystemLibrary.Delay` 0.75)
  (`self.Spawn_mid_board2`)
  (`KismetSystemLibrary.Delay` 0.75)
  (`self.Spawn_mid_board2`)
  (`self.Spawn_mid_board3`)
  (`KismetSystemLibrary.Delay` 0.75)
  (`self.Spawn_mid_board3`)
  (`KismetSystemLibrary.Delay` 0.75)
  (`self.Spawn_mid_board3`)
  (`self.Spawn_top_board`)
  (`KismetSystemLibrary.Delay` 0.75)
  (`self.Spawn_top_board`)
  (`KismetSystemLibrary.Delay` 0.75)
  (`self.Spawn_top_board`))

(event `self.Box.OnComponentBeginOverlap`
  (params (OverlappedComponent :type "PrimitiveComponent Object Reference") (OtherActor :type "Actor Object Reference") (OtherComp :type "PrimitiveComponent Object Reference") (OtherBodyIndex :type Integer) (bFromSweep :type Boolean) (SweepResult :type "HitResult Structure (by ref)"))
  (cast `/Game/ThirdPersonBP/Blueprints/ThirdPersonCharacter` OtherActor)
  (bind _asthird_person_game_mode (cast `/Game/ThirdPersonBP/Blueprints/ThirdPersonGameMode` (`GameplayStatics.GetGameMode`)))
  (`/Game/ThirdPersonBP/Blueprints/ThirdPersonGameMode.Spawn_tile` _asthird_person_game_mode)
  (bind _asthird_person_game_mode_2 (cast `/Game/ThirdPersonBP/Blueprints/ThirdPersonGameMode` (`GameplayStatics.GetGameMode`)))
  (set `/Game/ThirdPersonBP/Blueprints/ThirdPersonGameMode.currentPoint` (+ (* 1 (`/Game/ThirdPersonBP/Blueprints/ThirdPersonGameMode.PointMultiplier` _asthird_person_game_mode_2)) (`/Game/ThirdPersonBP/Blueprints/ThirdPersonGameMode.currentPoint` _asthird_person_game_mode_2)) _asthird_person_game_mode_2))

(event `self.Box1.OnComponentBeginOverlap`
  (params (OverlappedComponent :type "PrimitiveComponent Object Reference") (OtherActor :type "Actor Object Reference") (OtherComp :type "PrimitiveComponent Object Reference") (OtherBodyIndex :type Integer) (bFromSweep :type Boolean) (SweepResult :type "HitResult Structure (by ref)"))
  (cast `/Game/ThirdPersonBP/Blueprints/ThirdPersonCharacter` OtherActor)
  (cast `/Game/ThirdPersonBP/Blueprints/ThirdPersonGameMode` (`GameplayStatics.GetGameMode`))
  (`self.Spawn_train`)
  (`GameplayStatics.PlaySound2D` "/Game/runner_filer/sound/train_honk_sound.train_honk_sound" 1.0 1.0 0.0 null null))

(fn `Spawn money`
  ;[1 1 1] left_lane1
  (switch `int` (`KismetMathLibrary.RandomIntegerInRange` 0 3)
    (:`0`
      (`|SpawnActorFromClass` "/Game/runner_filer/blueprint/coin_pickup.coin_pickup_C" (`SceneComponent.K2_GetComponentToWorld` (`self.left_lane1`)) "Undefined" "OverrideRootScale" null null))
    (:`1`
      ;[1 1 1] center_lane
      (`|SpawnActorFromClass` "/Game/runner_filer/blueprint/coin_pickup.coin_pickup_C" (`SceneComponent.K2_GetComponentToWorld` (`self.center_lane`)) "Undefined" "OverrideRootScale" null null))
    (:`2`
      ;[1 1 1] right_lane1
      (`|SpawnActorFromClass` "/Game/runner_filer/blueprint/coin_pickup.coin_pickup_C" (`SceneComponent.K2_GetComponentToWorld` (`self.right_lane1`)) "Undefined" "OverrideRootScale" null null))))

(fn `Spawn_bot_board`
  ;[1 1 1] left_lane1
  (`|SpawnActorFromClass` "/Game/runner_filer/blueprint/left_board.left_board_C" (`SceneComponent.K2_GetComponentToWorld` (`self.water_left1`)) "Undefined" "OverrideRootScale" null null))

(fn `Spawn_bot_car`
  ;[1 1 1] left_lane1
  (switch `int` (`KismetMathLibrary.RandomIntegerInRange` 0 2)
    (:`1`
      (`|SpawnActorFromClass` "/Game/runner_filer/blueprint/blue_car.blue_car_C" (`SceneComponent.K2_GetComponentToWorld` (`self.bot_lane_right`)) "Undefined" "OverrideRootScale" null null))))

(fn `Spawn_mid_board1`
  ;[1 1 1] left_lane1
  (`|SpawnActorFromClass` "/Game/runner_filer/blueprint/right_board.right_board_C" (`SceneComponent.K2_GetComponentToWorld` (`self.water_mid_right1`)) "Undefined" "OverrideRootScale" null null))

(fn `Spawn_mid_board2`
  ;[1 1 1] left_lane1
  (`|SpawnActorFromClass` "/Game/runner_filer/blueprint/left_board.left_board_C" (`SceneComponent.K2_GetComponentToWorld` (`self.water_mid_left2`)) "Undefined" "OverrideRootScale" null null))

(fn `Spawn_mid_board3`
  ;[1 1 1] left_lane1
  (`|SpawnActorFromClass` "/Game/runner_filer/blueprint/right_board.right_board_C" (`SceneComponent.K2_GetComponentToWorld` (`self.water_mid_Right3`)) "Undefined" "OverrideRootScale" null null))

(fn `Spawn_top_board`
  ;[1 1 1] left_lane1
  (`|SpawnActorFromClass` "/Game/runner_filer/blueprint/left_board.left_board_C" (`SceneComponent.K2_GetComponentToWorld` (`self.water_top_left`)) "Undefined" "OverrideRootScale" null null))

(fn `Spawn_top_car`
  ;[1 1 1] left_lane1
  (switch `int` (`KismetMathLibrary.RandomIntegerInRange` 0 2)
    (:`0`
      (`|SpawnActorFromClass` "/Game/runner_filer/blueprint/car2.car2_C" (`SceneComponent.K2_GetComponentToWorld` (`self.left_lane1`)) "Undefined" "OverrideRootScale" null null))
    (:`1`
      (`|SpawnActorFromClass` "/Game/runner_filer/blueprint/car1.car1_C" (`SceneComponent.K2_GetComponentToWorld` (`self.left_lane1`)) "Undefined" "OverrideRootScale" null null))))

(fn `Spawn_train`
  ;[1 1 1] left_lane1
  (switch `int` (`KismetMathLibrary.RandomIntegerInRange` 0 1)
    (:`0`
      (`|SpawnActorFromClass` "/Game/runner_filer/blueprint/left_right_train.left_right_train_C" (`SceneComponent.K2_GetComponentToWorld` (`self.left_train`)) "Undefined" "OverrideRootScale" null null))
    (:`1`
      ;[1 1 1] center_lane
      (`|SpawnActorFromClass` "/Game/runner_filer/blueprint/right_left_train.right_left_train_C" (`SceneComponent.K2_GetComponentToWorld` (`self.right_train`)) "Undefined" "OverrideRootScale" null null))))

(fn `spawn_water`
  ;[1 1 1] left_lane1
  (`|SpawnActorFromClass` "/Game/runner_filer/blueprint/ocean_obstacle.ocean_obstacle_C" (`SceneComponent.K2_GetComponentToWorld` (`self.center water`)) "Undefined" "OverrideRootScale" null null))

(fn `UserConstructionScript`)