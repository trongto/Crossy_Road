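; Train tile for a lane-based endless runner that fills its lanes with a random obstacle and a possible coin pickup.
; On BeginPlay it spawns one car or ocean obstacle at a left, center or right lane point, and independently rolls for a coin, which can share that point.
; When the player character overlaps its box, it has the game mode spawn the next tile and adds multiplier-scaled points.
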(event `self.ReceiveBeginPlay`
  (`self.Spawn_obstacle`)
  (`self.Spawn money`))

(event `self.Box.OnComponentBeginOverlap`
  (params (OverlappedComponent :type "PrimitiveComponent Object Reference") (OtherActor :type "Actor Object Reference") (OtherComp :type "PrimitiveComponent Object Reference") (OtherBodyIndex :type Integer) (bFromSweep :type Boolean) (SweepResult :type "HitResult Structure (by ref)"))
  (cast `/Game/ThirdPersonBP/Blueprints/ThirdPersonCharacter` OtherActor)
  (bind _asthird_person_game_mode (cast `/Game/ThirdPersonBP/Blueprints/ThirdPersonGameMode` (`GameplayStatics.GetGameMode`)))
  (`/Game/ThirdPersonBP/Blueprints/ThirdPersonGameMode.Spawn_tile` _asthird_person_game_mode)
  (bind _asthird_person_game_mode_2 (cast `/Game/ThirdPersonBP/Blueprints/ThirdPersonGameMode` (`GameplayStatics.GetGameMode`)))
  (set `/Game/ThirdPersonBP/Blueprints/ThirdPersonGameMode.currentPoint` (+ (* 1 (`/Game/ThirdPersonBP/Blueprints/ThirdPersonGameMode.PointMultiplier` _asthird_person_game_mode_2)) (`/Game/ThirdPersonBP/Blueprints/ThirdPersonGameMode.currentPoint` _asthird_person_game_mode_2)) _asthird_person_game_mode_2))

(fn `Spawn money`
  ;[1 1 1] left_lane1
  (switch `int` (`KismetMathLibrary.RandomIntegerInRange` 0 3)
    (:`0`
      (`|SpawnActorFromClass` "/Game/runner_filer/blueprint/coin_pickup.coin_pickup_C" (`SceneComponent.K2_GetComponentToWorld` (`self.left_lane1`)) "Undefined" "OverrideRootScale" null null))
    (:`1`
      ;[1 1 1] center_lane
      (`|SpawnActorFromClass` "/Game/runner_filer/blueprint/coin_pickup.coin_pickup_C" (`SceneComponent.K2_GetComponentToWorld` (`self.center_lane`)) "Undefined" "OverrideRootScale" null null))
    (:`2`
      ;[1 1 1] right_lane1
      (`|SpawnActorFromClass` "/Game/runner_filer/blueprint/coin_pickup.coin_pickup_C" (`SceneComponent.K2_GetComponentToWorld` (`self.right_lane1`)) "Undefined" "OverrideRootScale" null null))))

(fn `Spawn_obstacle`
  (bind _returnvalue (`SceneComponent.K2_GetComponentToWorld` (`self.right_lane1`)))
  (bind _returnvalue_2 (`SceneComponent.K2_GetComponentToWorld` (`self.left_lane1`)))
  ;[1 1 1] left_lane1
  (switch `int` (`KismetMathLibrary.RandomIntegerInRange` 0 4)
    (:`0`
      (`|SpawnActorFromClass` "/Game/runner_filer/blueprint/car1.car1_C" _returnvalue_2 "Undefined" "OverrideRootScale" null null))
    (:`1`
      (`|SpawnActorFromClass` "/Game/runner_filer/blueprint/ocean_obstacle.ocean_obstacle_C" _returnvalue_2 "Undefined" "OverrideRootScale" null null))
    (:`2`
      ;[1 1 1] center_lane
      (`|SpawnActorFromClass` "/Game/runner_filer/blueprint/ocean_obstacle.ocean_obstacle_C" (`SceneComponent.K2_GetComponentToWorld` (`self.center_lane`)) "Undefined" "OverrideRootScale" null null))
    (:`3`
      ;[1 1 1] right_lane1
      (`|SpawnActorFromClass` "/Game/runner_filer/blueprint/ocean_obstacle.ocean_obstacle_C" _returnvalue "Undefined" "OverrideRootScale" null null))
    (:`4`
      (`|SpawnActorFromClass` "/Game/runner_filer/blueprint/blue_car.blue_car_C" _returnvalue "Undefined" "OverrideRootScale" null null))))

(fn `UserConstructionScript`)